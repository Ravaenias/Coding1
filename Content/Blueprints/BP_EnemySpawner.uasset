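; Enemy spawner actor that populates placed BP_EnemySpawnLocation markers with BP_Enemy.
; On BeginPlay it gathers the markers, prints their count on screen, then rolls a weighted chance at each one to spawn an enemy there.
; A self-recalling check with a two-second delay polls for living enemies via GetAllActorsOfClass and runs another spawn wave when none remain.
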(event Custom|Spawn%20Enemies
  (for _array_element (stale EventBeginPlay _outactors)
    (if (Math|Random|RandomBoolwithWeight 0.5)
      (Game|SpawnActorfromClass "/Game/Blueprints/BP_Enemy.BP_Enemy_C" (Transformation|GetActorTransform _array_element) "Undefined" "MultiplyWithRoot" 0 0) ; Spawn actor from class
    )))

(event Custom|Check%20Enemy
  (bind _outactors (Actor|GetAllActorsOfClass "/Game/Blueprints/BP_Enemy.BP_Enemy_C")) ; Expensive
  (if (> (Utilities|Array|Length _outactors) 0)
    _
    (else
      (CallFunction|SpawnEnemies)))
  (Utilities|FlowControl|Delay 2.0)
  (CallFunction|CheckEnemy))

(event EventBeginPlay
  (bind _outactors (Actor|GetAllActorsOfClass "/Game/Blueprints/BP_EnemySpawnLocation.BP_EnemySpawnLocation_C"))
  (Development|PrintString (Utilities|String|Append "There are" (Utilities|String|ToString(Integer) (Utilities|Array|Length _outactors)) " spawn locations") true true "(R=0.522569,G=0.000000,B=0.010813,A=1.000000)" 1e+01)
  (CallFunction|SpawnEnemies)
  (CallFunction|CheckEnemy))

(fn ConstructionScript)