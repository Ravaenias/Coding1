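; BP_Item is a game item that sets its damage by type and can subtract it from an enemy's health.
; On BeginPlay, Constructor rolls random damage and any missing name for weapons, while tools and consumables get fixed damage.
; It then prints name and damage, waits briefly, and calls Attack on a BP_Enemy found through GetActorOfClass.
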(event EventBeginPlay
  (CallFunction|Constructor)
  (Development|PrintString (Utilities|String|Append "Name:" (Variables|Default|GetName) "Damage:" (Utilities|String|ToString(Integer) (Variables|Default|GetDamage))))
  (Utilities|FlowControl|Delay 5.0)
  (bind _returnvalue (Actor|GetActorOfClass "/Game/Blueprints/BP_Enemy.BP_Enemy_C"))
  (CallFunction|Attack _returnvalue))

(fn ConstructionScript)

(fn Constructor
  (bind _weaponnames (Variables|Default|GetWeaponNames))
  (switch Utilities|FlowControl|Switch|SwitchonItemType (Variables|Default|GetType)
    (:NewEnumerator0
      (Variables|Default|SetDamage (Math|Random|RandomIntegerinRange 3 6))
      (if (Utilities|Enum|Equal(Enum) (Variables|Default|GetName) "") ; if true, randomize name\nif false, already has name
        (Utilities|Array|Shuffle _weaponnames) ; shuffle the list
        (Variables|Default|SetName (Utilities|Array|Get(acopy) _weaponnames))))
    (:NewEnumerator1
      (Variables|Default|SetDamage 1))
    (:NewEnumerator2
      (Variables|Default|SetDamage 0))))

(fn Attack
  (params (GivenEnemy :type BP%20Enemy%20Object%20Reference))
  (Variables|/Game/Blueprints/BP_Enemy.BP_Enemy_C|SetHealth GivenEnemy (- (Variables|/Game/Blueprints/BP_Enemy.BP_Enemy_C|GetHealth GivenEnemy) (Variables|Default|GetDamage))) ; set health
)